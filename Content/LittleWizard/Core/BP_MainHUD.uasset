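; Main HUD for LittleWizard that manages the location screens and the points and gold overlay.
; On BeginPlay it creates the Map and Cabinet widgets, opens the Map and sets UI-only input with a visible cursor.
; SetCurrentOpenedWidget swaps the screen and recreates WBP_HUD on top each time.
; Points and gold events and getters pass straight through to that HUD widget, which holds the values.
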(event `self.ReceiveBeginPlay`
  (`self.CreateWidgetLocations`) ; ПОД ВОПРОСОМ ФУНКЦИЯ\n\nВОЗМОЖНО СТОИТ КРЕЕТИТЬ ТОЛЬКО СТАРТ ЛОКАЦИЮ\nА ВСЕ ОСТАЛЬНЫЕ ПРОСТО ПЕРЕДАВАТЬ ДЛЯ ДОБАВЛЕНИЯ НА ЭКРАН\n(НЕОБХОДИМУЮ ЛОГИКУ ДРУГИХ ВИДЖЕТОВ ВЕСТИ ЧЕРЕЗ АКТОР КОМПОНЕНТЫ)
  (`self.SetCurrentOpenedWidget` (`self.WidgetMap`)) ; ТУТ ДВОЙНАЯ ЛОГИКА - В ПРЕДЫДУЩЕЙ ФУНКЦИИ Я СТАВЛЮ ВИДЖЕТ\nА В ЭТОЙ ОПЯТЬ ЕГО ПОЛУЧАЮ, ПОТОМ УДАЛЯЮ И ОПЯТЬ ДОБАВЛЯЮ
  (`WidgetBlueprintLibrary.SetInputMode_UIOnlyEx` (`self.GetOwningPlayerController`) null)
  (set `PlayerController.bShowMouseCursor` true (`self.GetOwningPlayerController`)))

(event `OnSetPlayerPoints`
  (params (NewPoints :type Integer))
  (bind _widgethud (`self.WidgetHUD`))
  (`/Engine/EditorBlueprintResources/StandardMacros.IsValid` _widgethud
    (:`Is Valid`
      (`/Game/LittleWizard/Core/UI/WBP_HUD.SetCurrentPoints` _widgethud NewPoints))))

(event `OnSetPlayerGold`
  (params (NewGold :type Integer))
  (bind _widgethud (`self.WidgetHUD`))
  (`/Engine/EditorBlueprintResources/StandardMacros.IsValid` _widgethud
    (:`Is Valid`
      (`/Game/LittleWizard/Core/UI/WBP_HUD.SetCurrentGold` _widgethud NewGold))))

(fn `CreateWidgetLocations`
  (bind _returnvalue (`|CreateWidget` "/Game/LittleWizard/Core/UI/Locations/WBP_Map.WBP_Map_C" (`self.GetOwningPlayerController`)))
  (set `self.WidgetMap` _returnvalue)
  (bind _returnvalue_2 (`|CreateWidget` "/Game/LittleWizard/Core/UI/Locations/Cabinet/WBP_Cabinet.WBP_Cabinet_C" (`self.GetOwningPlayerController`)))
  (set `self.WidgetCabinet` _returnvalue_2)
  (return))

(fn `GetCurrentGold`
  (returns (CurrentGold :type Integer))
  (bind _widgethud (`self.WidgetHUD`))
  (`/Engine/EditorBlueprintResources/StandardMacros.IsValid` _widgethud
    (:`Is Valid`
      (bind _goldcount (`/Game/LittleWizard/Core/UI/WBP_HUD.GetCurrentGold` _widgethud))
      (return _goldcount))))

(fn `GetCurrentOpenedWidget`
  (returns (OpenedWidget :type "UserWidget Object Reference"))
  (return (`self.CurrentOpenedWidget`)))

(fn `GetCurrentPoints`
  (returns (CurrentPoints :type Integer))
  (bind _widgethud (`self.WidgetHUD`))
  (`/Engine/EditorBlueprintResources/StandardMacros.IsValid` _widgethud
    (:`Is Valid`
      (bind _pointscount (`/Game/LittleWizard/Core/UI/WBP_HUD.GetCurrentPoints` _widgethud))
      (return _pointscount))))

(fn `SetCurrentOpenedWidget`
  (params (CurrentWidget :type "UserWidget Object Reference"))
  (bind _openedwidget (`self.GetCurrentOpenedWidget`))
  (`/Engine/EditorBlueprintResources/StandardMacros.IsValid` _openedwidget
    (:`Is Valid`
      (`Widget.RemoveFromParent` _openedwidget))
    (:`Is Not Valid`
      _))
  (`/Engine/EditorBlueprintResources/StandardMacros.IsValid` (`self.WidgetHUD`)
    (:`Is Valid`
      (`Widget.RemoveFromParent` (`self.WidgetHUD`)))
    (:`Is Not Valid`
      _))
  (bind _output_get (set `self.CurrentOpenedWidget` (`local.CurrentWidget`)))
  (`UserWidget.AddToViewport` _output_get 0)
  (bind _returnvalue (`|CreateWidget` "/Game/LittleWizard/Core/UI/WBP_HUD.WBP_HUD_C" (`self.GetOwningPlayerController`)))
  (bind _output_get_2 (set `self.WidgetHUD` _returnvalue))
  (`UserWidget.AddToViewport` _output_get_2 0)
  (return))

(fn `UserConstructionScript`)