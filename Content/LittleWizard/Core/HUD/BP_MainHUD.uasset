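; Main HUD class for LittleWizard that shows the main menu on BeginPlay with UI-only input and a visible cursor.
; It binds the menu's Play, Continue and Exit events: Play swaps the menu for the in-game HUD widget, Exit quits, and Continue is an empty stub.
; Helper functions create or remove both widgets and return the HUD widget's current magic power count, or zero if that widget is invalid.
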(event `self.ReceiveBeginPlay`
  (bind _mainmenuwidget (`self.OpenMainMenuWidget` self))
  (`self.OnOpenedMainMenu` self _mainmenuwidget)
  (`WidgetBlueprintLibrary.SetInputMode_UIOnlyEx` (`self.GetOwningPlayerController` self) null)
  (set `PlayerController.bShowMouseCursor` true (`self.GetOwningPlayerController` self)))

(event `OnOpenedMainMenu`
  (params (MainMenuWidget :type "/Game/LittleWizard/Core/UI/Menu/WBP_MainMenu Object Reference"))
  (add `/Game/LittleWizard/Core/UI/Menu/WBP_MainMenu.OnPlayButtonPressed` MainMenuWidget (delegate `OnPlayButtonPressed`))
  (add `/Game/LittleWizard/Core/UI/Menu/WBP_MainMenu.OnContinueButtonPressed` (`self.MainMenuWidget`) (delegate `OnContinueButtonPressed`))
  (add `/Game/LittleWizard/Core/UI/Menu/WBP_MainMenu.OnExitButtonPressed` (`self.MainMenuWidget`) (delegate `OnExitButtonPressed`)))

(event `OnPlayButtonPressed`
  (`self.OpenHUDWidget` self)
  (`self.RemoveMainMenuWidget` self))

(event `OnContinueButtonPressed`)

(event `OnExitButtonPressed`
  (`KismetSystemLibrary.QuitGame` (`self.GetOwningPlayerController` self) "Quit"))

(fn `GetCurrentCountMagicPowerInHUD`
  (returns (MagicPowerCurrentValue :type Integer))
  (bind _hudwidget (`self.HUDWidget`))
  (`/Engine/EditorBlueprintResources/StandardMacros.IsValid` _hudwidget
    (:`Is Valid`
      (bind _magicpowercurrentvalue (`/Game/LittleWizard/Core/UI/WBP_HUD.GetCurrentCountMagicPower` _hudwidget))
      (return _magicpowercurrentvalue))
    (:`Is Not Valid`
      (return 0))))

(fn `OpenHUDWidget`
  (returns (HUDWidget :type "/Game/LittleWizard/Core/UI/WBP_HUD Object Reference"))
  (bind _returnvalue (`|CreateWidget` "/Game/LittleWizard/Core/UI/WBP_HUD.WBP_HUD_C" (`self.GetOwningPlayerController` self)))
  (bind _output_get (set `self.HUDWidget` _returnvalue))
  (`UserWidget.AddToViewport` _output_get 0)
  (return (`self.HUDWidget`)))

(fn `OpenMainMenuWidget`
  (returns (MainMenuWidget :type "/Game/LittleWizard/Core/UI/Menu/WBP_MainMenu Object Reference"))
  (bind _returnvalue (`|CreateWidget` "/Game/LittleWizard/Core/UI/Menu/WBP_MainMenu.WBP_MainMenu_C" (`self.GetOwningPlayerController` self)))
  (bind _output_get (set `self.MainMenuWidget` _returnvalue))
  (`UserWidget.AddToViewport` _output_get 0)
  (return (`self.MainMenuWidget`)))

(fn `RemoveHUDWidget`
  (`Widget.RemoveFromParent` (`self.HUDWidget`))
  (return))

(fn `RemoveMainMenuWidget`
  (`Widget.RemoveFromParent` (`self.MainMenuWidget`))
  (return))

(fn `UserConstructionScript`)